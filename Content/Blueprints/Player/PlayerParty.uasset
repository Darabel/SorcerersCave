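; PlayerParty is the pawn or actor representing the party on a tile grid, starting at the "Entrance"-tagged tile with a randomly blue-tinted sprite.
; MovePlayer checks exits on both tiles, gets the neighbor through MyGameState's RequireTileAt, records the previous tile, teleports, then notifies the tile and player controller.
; CurrentTile's RepNotify broadcasts EnteredRoom when the new tile is a room.
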(event `self.ReceiveBeginPlay`
  (set `self.PlayerParty` (`/Game/Blueprints/Game/MyPartyGameInstance.PartyMembers` (cast `/Game/Blueprints/Game/MyPartyGameInstance` (`GameplayStatics.GetGameInstance`) :!pure true)))
  (`PaperSpriteComponent.SetSpriteColor` (`self.PaperSprite`) (make `LinearColor` 0.0 0.0 (`KismetMathLibrary.RandomFloatInRange` 0.0 1.0) 1.0))
  (bind _outactors (`GameplayStatics.GetAllActorsWithTag` "Entrance"))
  (set `self.CurrentTile` (cast `/Game/Blueprints/Map/Tile` (`|GetArrayItem` _outactors) :!pure true)))

(event `MovePlayer`
  (params (Direction :type "Vector Structure"))
  (bind _currenttile (`self.CurrentTile`))
  (bind _canmove (`/Game/Blueprints/Map/Tile.CanMove` _currenttile Direction))
  (if _canmove
    (bind _tile (`/Game/Blueprints/Game/MyGameState.RequireTileAt` (cast `/Game/Blueprints/Game/MyGameState` (`GameplayStatics.GetGameState`) :!pure true) (+ (`/Game/Blueprints/Map/Tile.GetGridLocation` _currenttile) Direction)))
    (bind _canmove_2 (`/Game/Blueprints/Map/Tile.CanMove` _tile (`KismetMathLibrary.NegateVector` Direction)))
    (if _canmove_2
      (`KismetArrayLibrary.Array_Add` (`self.LastTile`) (`self.CurrentTile`))
      (bind _output_get (set `self.CurrentTile` _tile))
      (bind (_returnvalue_x _returnvalue_y _returnvalue_z) (`KismetMathLibrary.BreakVector` (`self.K2_GetActorLocation` _output_get)))
      (`self.K2_SetActorLocation` (`KismetMathLibrary.MakeVector` _returnvalue_x (+ _returnvalue_y 1.0) _returnvalue_z) false true)
      (`/Game/Blueprints/Map/Tile.PlayerEntered` _output_get)
      (`/Game/Blueprints/Player/MyPlayerController.MovedPlayer_Event` (cast `/Game/Blueprints/Player/MyPlayerController` (`GameplayStatics.GetPlayerController` 0) :!pure true)))))

(fn `OnRep_CurrentTile`
  (bind _currenttile (`self.CurrentTile`))
  (`/Engine/EditorBlueprintResources/StandardMacros.IsValid` _currenttile
    (:`Is Valid`
      (if (`/Game/Blueprints/Map/Tile.IsRoom` _currenttile)
        (`self.EnteredRoom` _currenttile)))
    (:`Is Not Valid`
      (`KismetSystemLibrary.PrintString` "NOT VALID CURRENT TILE" true true (struct :`R` 1.0 :`G` 0.092374 :`B` 0.232241 :`A` 1.0)))))

(fn `UserConstructionScript`)