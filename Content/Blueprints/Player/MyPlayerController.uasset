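; Player controller that turns directional input actions into movement of the controlled PlayerParty pawn.
; Each press of the four move actions casts the pawn and calls MovePlayer with a unit direction on the X or Z axis.
; MovedPlayer_Event prints a debug string, then calls MovedPlayer.
; HandleCardEvent only prints the received action.
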(event `InputAction|MoveUp`
  (params (Key :type "Key Structure"))
  (:`Pressed`
    (`/Game/Blueprints/Player/PlayerParty.MovePlayer` (cast `/Game/Blueprints/Player/PlayerParty` (`self.K2_GetPawn`) :!pure true) (0.0 0.0 1.0))))

(event `InputAction|MoveDown`
  (params (Key :type "Key Structure"))
  (:`Pressed`
    (`/Game/Blueprints/Player/PlayerParty.MovePlayer` (cast `/Game/Blueprints/Player/PlayerParty` (`self.K2_GetPawn`) :!pure true) (0.0 0.0 -1.0))))

(event `InputAction|MoveLeft`
  (params (Key :type "Key Structure"))
  (:`Pressed`
    (`/Game/Blueprints/Player/PlayerParty.MovePlayer` (cast `/Game/Blueprints/Player/PlayerParty` (`self.K2_GetPawn`) :!pure true) (-1.0 0.0 0.0))))

(event `MovedPlayer_Event`
  (`KismetSystemLibrary.PrintString` "Hello")
  (`self.MovedPlayer`))

(event `InputAction|MoveRight`
  (params (Key :type "Key Structure"))
  (:`Pressed`
    (`/Game/Blueprints/Player/PlayerParty.MovePlayer` (cast `/Game/Blueprints/Player/PlayerParty` (`self.K2_GetPawn`) :!pure true) (1.0 0.0 0.0))))

(event `HandleCardEvent`
  (params (Card :type "/Game/Data/Card Structure") (Action :type Name))
  (`KismetSystemLibrary.PrintString` (`KismetStringLibrary.Conv_NameToString` Action)))

(fn `UserConstructionScript`)