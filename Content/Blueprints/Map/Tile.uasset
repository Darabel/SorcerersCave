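; Map tile for a 2D grid dungeon with card encounters, shown as a passage, junction or room sprite.
; The authority picks a weighted random type for Unknown tiles at construction; Type drives sprite, rotation and which directions CanMove allows.
; First entry into a room deals level-based cards from the game instance and shows them on the HUD, with a RoomEntered RepNotify triggering card handling.
; HandleCards tallies card types into a summary widget.
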(event `self.ReceiveBeginPlay`
  (`KismetSystemLibrary.PrintString` (`|GetEnumeratorNameAsString` (`self.Type`)) true true (struct :`R` 0.20501 :`G` 1.0 :`B` 0.128417 :`A` 1.0) 12.0)
  (`self.SetSprite`))

(event `PlayerEntered`
  (bind _room (`self.IsRoom`))
  (if _room
    (if (`self.RoomEntered`)
      (`KismetSystemLibrary.PrintString` "Already Entered")
      (else
        (bind _dealtcards (`/Game/Blueprints/Game/MyPartyGameInstance.DealCards` (cast `/Game/Blueprints/Game/MyPartyGameInstance` (`GameplayStatics.GetGameInstance`) :!pure true) (`self.CurrentLevel`)))
        (set `self.RoomCards` _dealtcards)
        (set `self.RoomEntered` true)
        (`KismetSystemLibrary.PrintString` "Im a Room")))
    (`/Game/MyGameHUD.ShowRoomCards` (cast `/Game/MyGameHUD` (`PlayerController.GetHUD` (`GameplayStatics.GetPlayerController` 0)) :!pure true) (`self.RoomCards`))
    (else
      (`KismetSystemLibrary.PrintString` "Not a Room"))))

(fn `CanMove`
  (params (Direction :type "Vector Structure"))
  (returns (CanMove :type Boolean))
  (locals (Result :type Boolean))
  (`|ExecutionSequence`
    (:`then_0`
      (if (> Direction_Z 0.0)
        (switch `/Game/Data/ETileType` (`self.Type`)
          (:`NewEnumerator1`
            _)
          (:`NewEnumerator3`
            _)
          (:`NewEnumerator5`
            _)
          (:`NewEnumerator10`
            _)
          (:`NewEnumerator11`
            _)
          (:`NewEnumerator7`
            _)
          (:`NewEnumerator6`
            _)
          (:`NewEnumerator13`
            _)
          (:`NewEnumerator14`
            _)
          (:`NewEnumerator16`
            _)
          (:`NewEnumerator17`
            _))
        (set `local.Result` true)))
    (:`then_1`
      (if (< Direction_Z 0.0)
        (switch `/Game/Data/ETileType` (`self.Type`)
          (:`NewEnumerator1`
            _)
          (:`NewEnumerator3`
            _)
          (:`NewEnumerator4`
            _)
          (:`NewEnumerator10`
            _)
          (:`NewEnumerator11`
            _)
          (:`NewEnumerator9`
            _)
          (:`NewEnumerator8`
            _)
          (:`NewEnumerator13`
            _)
          (:`NewEnumerator15`
            _)
          (:`NewEnumerator16`
            _)
          (:`NewEnumerator17`
            _))
        (set `local.Result` true)))
    (:`then_2`
      (if (< Direction_X 0.0)
        (switch `/Game/Data/ETileType` (`self.Type`)
          (:`NewEnumerator1`
            _)
          (:`NewEnumerator2`
            _)
          (:`NewEnumerator4`
            _)
          (:`NewEnumerator5`
            _)
          (:`NewEnumerator10`
            _)
          (:`NewEnumerator7`
            _)
          (:`NewEnumerator9`
            _)
          (:`NewEnumerator13`
            _)
          (:`NewEnumerator14`
            _)
          (:`NewEnumerator15`
            _)
          (:`NewEnumerator16`
            _))
        (set `local.Result` true)))
    (:`then_3`
      (if (> Direction_X 0.0)
        (switch `/Game/Data/ETileType` (`self.Type`)
          (:`NewEnumerator1`
            _)
          (:`NewEnumerator2`
            _)
          (:`NewEnumerator4`
            _)
          (:`NewEnumerator5`
            _)
          (:`NewEnumerator11`
            _)
          (:`NewEnumerator6`
            _)
          (:`NewEnumerator8`
            _)
          (:`NewEnumerator13`
            _)
          (:`NewEnumerator14`
            _)
          (:`NewEnumerator15`
            _)
          (:`NewEnumerator17`
            _))
        (set `local.Result` true)))
    (:`then_4`
      (return (`local.Result`)))))

(fn `GetGridLocation`
  (returns (GridLocation :type "Vector Structure"))
  (return (/ (`self.K2_GetActorLocation`) (256.0 1.0 256.0))))

(fn `HandleCards`
  (locals (CardText :type String) (Hazards :type Integer) (Characters :type Integer) (SpecialCards :type Integer))
  (bind _cardtext (`local.CardText`))
  (for _array_element (`self.RoomCards`)
    (switch `name` (`.Type_45_179AC156426F3AA839B824802BCCBE0F` (break `/Game/Data/Card` _array_element))
      (:`Default`
        (set `local.CardText` (`KismetStringLibrary.Concat_StrStr` _cardtext "Somethng unknown is here.  "))
        (`/Engine/EditorBlueprintResources/StandardMacros.IncrementInt` (`local.SpecialCards`)))
      (:`Character`
        (set `local.CardText` (`KismetStringLibrary.Concat_StrStr` _cardtext "You have to test the stranger. "))
        (`/Engine/EditorBlueprintResources/StandardMacros.IncrementInt` (`local.Characters`)))
      (:`Treasure`
        (set `local.CardText` (`KismetStringLibrary.Concat_StrStr` _cardtext "Treasure.  ")))
      (:`Hazard`
        (set `local.CardText` (`KismetStringLibrary.Concat_StrStr` _cardtext "HAZARD.  "))
        (`/Engine/EditorBlueprintResources/StandardMacros.IncrementInt` (`local.Hazards`)))
      (:`Artefact`
        (set `local.CardText` (`KismetStringLibrary.Concat_StrStr` _cardtext "You have found an artefact.  ")))))
  (bind _returnvalue (`|CreateWidget` "/Game/Widgets/Rooms/CardHandling.CardHandling_C" null (`KismetTextLibrary.Conv_StringToText` (`local.CardText`))))
  (`UserWidget.AddToViewport` _returnvalue 0))

(fn `IsRoom`
  (returns (Room :type Boolean))
  (locals (IsARoom :type Boolean))
  (switch `/Game/Data/ETileType` (`self.Type`)
    (:`NewEnumerator13`
      _)
    (:`NewEnumerator14`
      _)
    (:`NewEnumerator15`
      _)
    (:`NewEnumerator16`
      _)
    (:`NewEnumerator17`
      _))
  (bind _output_get (set `local.IsARoom` true))
  (return _output_get))

(fn `OnRep_RoomEntered`
  (`/Game/MyGameHUD.HandleRoomCards` (cast `/Game/MyGameHUD` (`PlayerController.GetHUD` (`GameplayStatics.GetPlayerController` 0)) :!pure true) (`self.RoomCards`)))

(fn `SetSprite`
  (bind _papersprite (`self.PaperSprite`))
  (switch `/Game/Data/ETileType` (`self.Type`)
    (:`NewEnumerator1`
      (`PaperSpriteComponent.SetSprite` _papersprite "/Game/Graphics/Sprites/cross_sprite.cross_sprite")
      (`SceneComponent.K2_SetRelativeRotation` :`self` _papersprite :!label _label))
    (:`NewEnumerator2`
      (`PaperSpriteComponent.SetSprite` _papersprite "/Game/Graphics/Sprites/straight_sprite.straight_sprite")
      (goto _label))
    (:`NewEnumerator3`
      (`PaperSpriteComponent.SetSprite` _papersprite "/Game/Graphics/Sprites/passage_sprite.passage_sprite")
      (goto _label))
    (:`NewEnumerator4`
      (`PaperSpriteComponent.SetSprite` _papersprite "/Game/Graphics/Sprites/t_sprite.t_sprite")
      (goto _label))
    (:`NewEnumerator5`
      (`PaperSpriteComponent.SetSprite` _papersprite "/Game/Graphics/Sprites/t_sprite.t_sprite")
      (`SceneComponent.K2_SetRelativeRotation` _papersprite (struct :`Pitch` 180.0) false false :!label _label_2))
    (:`NewEnumerator10`
      (`PaperSpriteComponent.SetSprite` _papersprite "/Game/Graphics/Sprites/t_sprite.t_sprite")
      (`SceneComponent.K2_SetRelativeRotation` _papersprite (struct :`Pitch` 270.0) false false :!label _label_3))
    (:`NewEnumerator11`
      (`PaperSpriteComponent.SetSprite` _papersprite "/Game/Graphics/Sprites/t_sprite.t_sprite")
      (`SceneComponent.K2_SetRelativeRotation` _papersprite (struct :`Pitch` 90.0) false false :!label _label_4))
    (:`NewEnumerator7`
      (`PaperSpriteComponent.SetSprite` _papersprite "/Game/Graphics/Sprites/corner_sprite.corner_sprite")
      (goto _label_2))
    (:`NewEnumerator6`
      (`PaperSpriteComponent.SetSprite` _papersprite "/Game/Graphics/Sprites/corner_sprite.corner_sprite")
      (goto _label_4))
    (:`NewEnumerator9`
      (`PaperSpriteComponent.SetSprite` _papersprite "/Game/Graphics/Sprites/corner_sprite.corner_sprite")
      (goto _label_3))
    (:`NewEnumerator8`
      (`PaperSpriteComponent.SetSprite` _papersprite "/Game/Graphics/Sprites/corner_sprite.corner_sprite")
      (goto _label))
    (:`NewEnumerator13`
      (`PaperSpriteComponent.SetSprite` _papersprite "/Game/Graphics/Sprites/room4_sprite.room4_sprite")
      (goto _label))
    (:`NewEnumerator14`
      (`PaperSpriteComponent.SetSprite` _papersprite "/Game/Graphics/Sprites/room3_sprite.room3_sprite")
      (goto _label))
    (:`NewEnumerator15`
      (`PaperSpriteComponent.SetSprite` _papersprite "/Game/Graphics/Sprites/room3_sprite.room3_sprite")
      (goto _label_2))
    (:`NewEnumerator16`
      (`PaperSpriteComponent.SetSprite` _papersprite "/Game/Graphics/Sprites/room3_sprite.room3_sprite")
      (goto _label_4))
    (:`NewEnumerator17`
      (`PaperSpriteComponent.SetSprite` _papersprite "/Game/Graphics/Sprites/room3_sprite.room3_sprite")
      (goto _label_3))))

(fn `SetType`
  (if (`|EnumEquality` (`self.Type`) "NewEnumerator12")
    (if (`KismetMathLibrary.RandomBoolWithWeight` 0.6)
      (set `self.Type` (cast `/Game/Data/ETileType` (`KismetMathLibrary.Conv_IntToByte` (`KismetMathLibrary.RandomIntegerInRange` 1 11))))
      (else
        (set `self.Type` (cast `/Game/Data/ETileType` (`KismetMathLibrary.Conv_IntToByte` (`KismetMathLibrary.RandomIntegerInRange` 11 16))))))
    (`KismetSystemLibrary.PrintString` (`|GetEnumeratorNameAsString` (`self.Type`)) true true (struct :`R` 1.0 :`G` 0.970081 :`B` 0.199474 :`A` 1.0) 10.0)))

(fn `UserConstructionScript`
  (`/Engine/EditorBlueprintResources/ActorMacros.Switch Has Authority`
    (:`Authority`
      (`self.SetType`)
      (`self.SetSprite`))))