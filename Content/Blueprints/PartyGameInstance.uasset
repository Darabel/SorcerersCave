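; Party game instance that supplies the card deck for the game.
; GetDeck builds the Deck lazily from the CardsTable data table when it is empty, then returns it.
; Each found row is added as repeated copies according to its Quantity field, with rows of one or less added once.
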(fn `GetDeck`
  (returns (Deck :type "Array of /Game/Data/Card Structure"))
  (`|ExecutionSequence`
    (:`then_0`
      (if (== (`KismetArrayLibrary.Array_Length` (`self.Deck`)) 0)
        (bind _outrownames (`DataTableFunctionLibrary.GetDataTableRowNames` "/Game/Data/CardsTable.CardsTable"))
        (for _array_element _outrownames
          (bind _returnvalue (`|GetDataTableRow` "/Game/Data/CardsTable.CardsTable" _array_element)
            (:`then`
              (bind ((`Quantity_36_D515C85544FDB14CABF0F29CC5810630` _quantity)) (break `/Game/Data/Card` _returnvalue))
              (if (> _quantity 1)
                (for _ (range _quantity)
                  (`KismetArrayLibrary.Array_Add` (`self.Deck`) _returnvalue :!label _label))
                (else
                  (goto _label))))))))
    (:`then_1`
      (return (`self.Deck`)))))