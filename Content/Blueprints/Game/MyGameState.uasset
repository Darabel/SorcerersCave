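; Game state that keeps the registry of grid tiles and provides a six-sided dice roll.
; On BeginPlay it registers the actor tagged "Entrance" as the starting tile in a location-to-Tile map.
; RequireTileAt returns the tile at a grid location, or spawns and registers one on the XZ plane at 256-unit spacing, flagging whether it is new.
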(event `self.ReceiveBeginPlay`
  (bind _outactors (`GameplayStatics.GetAllActorsWithTag` "Entrance"))
  (`BlueprintMapLibrary.Map_Add` (`self.Map`) (0.0 0.0 0.0) (cast `/Game/Blueprints/Map/Tile` (`|GetArrayItem` _outactors) :!pure true)))

(fn `GetTileAt`
  (params (Location :type "Vector Structure"))
  (returns (Tile :type "/Game/Blueprints/Map/Tile Object Reference") (IsValid :type Boolean))
  (bind (_value _returnvalue) (`BlueprintMapLibrary.Map_Find` (`self.Map`) Location))
  (return _value _returnvalue))

(fn `RequireTileAt`
  (params (Location :type "Vector Structure"))
  (returns (Tile :type "/Game/Blueprints/Map/Tile Object Reference") (New :type Boolean))
  (locals (TempTile :type "/Game/Blueprints/Map/Tile Object Reference"))
  (bind (_tile _isvalid) (`self.GetTileAt` Location))
  (if _isvalid
    (set `local.TempTile` _tile)
    (else
      (bind _returnvalue (`|SpawnActorFromClass` "/Game/Blueprints/Map/Tile.Tile_C" (`KismetMathLibrary.Conv_VectorToTransform` (* Location (256.0 0.0 256.0))) "Undefined" "OverrideRootScale" null null))
      (`BlueprintMapLibrary.Map_Add` (`self.Map`) Location _returnvalue)
      (set `local.TempTile` _returnvalue)))
  (return (`local.TempTile`) (not _isvalid)))

(fn `RollDice`
  (returns (Dice :type Integer))
  (return (`KismetMathLibrary.RandomIntegerInRange` 1 6)))

(fn `UserConstructionScript`)