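; Game instance for a party card game, holding the party members and the card deck.
; On Init it seeds the party with Hero, Woman and Dwarf from CardsTable, giving the Dwarf Gold as inventory.
; GetDeck lazily builds the deck by Quantity, and ShuffleDeck randomises it.
; DealCards moves cards into an uncleared CardsDealt by level number, skipping alternate cards because it removes while indexing upward.
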(event `self.ReceiveInit`
  (bind _outrownames (`DataTableFunctionLibrary.GetDataTableRowNames` "/Game/Data/CardsTable.CardsTable"))
  (for _array_element _outrownames
    (if (== _array_element "Hero")
      (bind _returnvalue (`|GetDataTableRow` "/Game/Data/CardsTable.CardsTable" _array_element)
        (:`then`
          (bind (_displayname _image _type _priority _quantity _pointvalue _weight _strength _magic _hostile _indifferent _friendly _partyvalue _partytype _description) (break `/Game/Data/Card` _returnvalue))
          (`KismetArrayLibrary.Array_Add` (`self.PartyMembers`) (make `/Game/Data/PartyCard` 1 _displayname _image _type _priority _quantity _pointvalue _weight _strength _magic _partytype _description (`|MakeArray` (struct) :!type "/Game/Data/Card Structure")))
          (break)))))
  (for _array_element_2 _outrownames
    (if (== _array_element_2 "Woman")
      (bind _returnvalue_2 (`|GetDataTableRow` "/Game/Data/CardsTable.CardsTable" _array_element_2)
        (:`then`
          (bind (_displayname_2 _image_2 _type_2 _priority_2 _quantity_2 _pointvalue_2 _weight_2 _strength_2 _magic_2 _hostile_2 _indifferent_2 _friendly_2 _partyvalue_2 _partytype_2 _description_2) (break `/Game/Data/Card` _returnvalue_2))
          (`KismetArrayLibrary.Array_Add` (`self.PartyMembers`) (make `/Game/Data/PartyCard` 2 _displayname_2 _image_2 _type_2 _priority_2 _quantity_2 _pointvalue_2 _weight_2 _strength_2 _magic_2 _partytype_2 _description_2 (`|MakeArray` (struct) :!type "/Game/Data/Card Structure")))
          (break)))))
  (for _array_element_3 _outrownames
    (if (== _array_element_3 "Gold")
      (bind _returnvalue_3 (`|GetDataTableRow` "/Game/Data/CardsTable.CardsTable" _array_element_3)
        (:`then`
          (`KismetArrayLibrary.Array_Add` (`self.TempInvArray`) _returnvalue_3)
          (for _array_element_4 _outrownames
            (if (== _array_element_4 "Dwarf")
              (bind _returnvalue_4 (`|GetDataTableRow` "/Game/Data/CardsTable.CardsTable" _array_element_4)
                (:`then`
                  (bind (_displayname_3 _image_3 _type_3 _priority_3 _quantity_3 _pointvalue_3 _weight_3 _strength_3 _magic_3 _hostile_3 _indifferent_3 _friendly_3 _partyvalue_3 _partytype_3 _description_3) (break `/Game/Data/Card` _returnvalue_4))
                  (`KismetArrayLibrary.Array_Add` (`self.PartyMembers`) (make `/Game/Data/PartyCard` 3 _displayname_3 _image_3 _type_3 _priority_3 _quantity_3 _pointvalue_3 _weight_3 _strength_3 _magic_3 _partytype_3 _description_3 (`self.TempInvArray`) 25))
                  (break))))))))))

(fn `DealCards`
  (params (LevelNumber :type Integer))
  (returns (DealtCards :type "Array of /Game/Data/Card Structure"))
  (locals (CardsDealt :type "Array of /Game/Data/Card Structure"))
  (bind _deck (`self.Deck`))
  (for _index (range (+ LevelNumber 1))
    (`KismetArrayLibrary.Array_Add` (`local.CardsDealt`) (`|GetArrayItem` _deck _index))
    (`KismetArrayLibrary.Array_Remove` _deck _index))
  (for _array_element (`local.CardsDealt`)
    (`KismetSystemLibrary.PrintString` (`KismetTextLibrary.Conv_TextToString` (`.DisplayName_44_F9C830A74787EE16942863BACB42B7FF` (break `/Game/Data/Card` _array_element))) true true (struct :`G` 0.66 :`B` 1.0 :`A` 1.0) 15.0))
  (return (`local.CardsDealt`)))

(fn `GetDeck`
  (returns (Deck :type "Array of /Game/Data/Card Structure"))
  (`|ExecutionSequence`
    (:`then_0`
      (if (== (`KismetArrayLibrary.Array_Length` (`self.Deck`)) 0)
        (bind _outrownames (`DataTableFunctionLibrary.GetDataTableRowNames` "/Game/Data/CardsTable.CardsTable"))
        (for _array_element _outrownames
          (bind _returnvalue (`|GetDataTableRow` "/Game/Data/CardsTable.CardsTable" _array_element)
            (:`then`
              (bind ((`Type_52_179AC156426F3AA839B824802BCCBE0F` _type) (`Priority_51_30492C104206E088E5E9229EC3176823` _priority) (`Quantity_36_D515C85544FDB14CABF0F29CC5810630` _quantity)) (break `/Game/Data/Card` _returnvalue))
              (if (> _quantity 1)
                (for _ (range _quantity)
                  (`KismetArrayLibrary.Array_Add` (`self.Deck`) _returnvalue :!label _label))
                (else
                  (goto _label))))))))
    (:`then_1`
      (return (`self.Deck`)))))

(fn `ShuffleDeck`
  (`KismetArrayLibrary.Array_Shuffle` (`self.Deck`))
  (`KismetSystemLibrary.PrintString` (`KismetTextLibrary.Conv_TextToString` (`.DisplayName_44_F9C830A74787EE16942863BACB42B7FF` (break `/Game/Data/Card` (`|GetArrayItem` (`self.Deck`))))) true true (struct :`R` 0.953125 :`G` 0.120975 :`B` 0.873015 :`A` 1.0) 15.0))