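; Blueprint function library for a card game with room cards and a player party, holding card action handlers and an action lookup.
; Stranger test, attack, treasure, artefact and hazard handlers are placeholders that only print debug text, and HandleCards is empty.
; GetActionsForCard scans the CardActionsTable data table row by row and returns the actions from the first row matching the card type.
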(fn `ArtefactCard`
  (params (Card :type "/Game/Data/Card Structure") (RoomCards :type "Array of /Game/Data/Card Structure") (PartyMembers :type "Array of /Game/Data/PartyCard Structure"))
  (`KismetSystemLibrary.PrintString` null "Artefact"))

(fn `AttackCard`
  (params (Card :type "/Game/Data/Card Structure") (RoomCards :type "Array of /Game/Data/Card Structure") (PartyMembers :type "Array of /Game/Data/PartyCard Structure"))
  (`KismetSystemLibrary.PrintString` null "You Attack!!!!" true true (struct :`R` 1.0 :`G` 0.962442 :`B` 0.983531 :`A` 1.0)))

(fn `GetActionsForCard`
  (params (CardType :type "/Game/Data/CardTypeEnum Enum" :default "NewEnumerator0"))
  (returns (CurrentActionArray :type "Array of /Game/Data/ActionTypeEnum Enum"))
  (locals (CurrentCardsActions :type "Array of /Game/Data/ActionTypeEnum Enum"))
  (bind _outrownames (`DataTableFunctionLibrary.GetDataTableRowNames` "/Game/Data/CardActionsTable.CardActionsTable"))
  (for _array_element _outrownames
    (bind _returnvalue (`|GetDataTableRow` "/Game/Data/CardActionsTable.CardActionsTable" _array_element)
      (:`then`
        (if (`|EnumEquality` (break `/Game/Data/CardTypeActions` _returnvalue) CardType)
          (set `local.CurrentCardsActions` (`.Actions_8_2FC1B101420D968C4A9EAE87B8EEC915` (break `/Game/Data/CardTypeActions` _returnvalue)))
          (break)))))
  (return (`local.CurrentCardsActions`)))

(fn `HandleCards`
  (params (RoomCards :type "Array of /Game/Data/Card Structure") (PlayerParty :type "Array of /Game/Data/PartyCard Structure") (SelectedCard :type "/Game/Data/Card Structure") (CurrentAction :type "/Game/Data/ActionTypeEnum Enum" :default "NewEnumerator0")))

(fn `HazardCard`
  (params (Card :type "/Game/Data/Card Structure") (RoomCards :type "Array of /Game/Data/Card Structure") (PartyMembers :type "Array of /Game/Data/PartyCard Structure"))
  (`KismetSystemLibrary.PrintString` null "HAZARD" true true (struct :`R` 1.0 :`G` 0.065688 :`B` 0.412565 :`A` 1.0)))

(fn `TestStangerCard`
  (params (Card :type "/Game/Data/Card Structure") (RoomCards :type "Array of /Game/Data/Card Structure") (PartyMembers :type "Array of /Game/Data/PartyCard Structure"))
  (`KismetSystemLibrary.PrintString` null "You test the Stanger" true true (struct :`R` 1.0 :`G` 0.970537 :`B` 0.992634 :`A` 1.0)))

(fn `TreasureCard`
  (params (Card :type "/Game/Data/Card Structure") (RoomCards :type "Array of /Game/Data/Card Structure") (PartyMembers :type "Array of /Game/Data/PartyCard Structure"))
  (`KismetSystemLibrary.PrintString` null "Treasure"))